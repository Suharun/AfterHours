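; BP_Key is a pickup key that the player can look at and interact with to gain a key.
; Overlapping the key caches the BP_Player reference, which InteractWith requires before destroying the key, setting HasKey on the player and playing a 2D pickup sound.
; LookAt and StopLookAt extend parent behavior by toggling the mesh's custom depth stencil value as a highlight while the key is interactable.
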(event `self.ReceiveActorBeginOverlap`
  (params (OtherActor :type "Actor Object Reference"))
  (`parent.ReceiveActorBeginOverlap` OtherActor)
  (bind _asbp_player (cast `/Game/Blueprints/BP_Player` OtherActor))
  (set `self.Player` _asbp_player))

(fn `InteractWith`
  (returns (Return :type Boolean))
  (if (`KismetSystemLibrary.IsValid` (`self.Player`))
    (`self.K2_DestroyActor`)
    (set `/Game/Blueprints/BP_Player.HasKey` true (`self.Player`))
    (bind _returnvalue (`GameplayStatics.CreateSound2D` "/Game/SFX/After_Hours_VA_-_Key_Found.After_Hours_VA_-_Key_Found" 1.0 1.0 0.0 null))
    (`AudioComponent.Play` _returnvalue 0.0)
    (return false)))

(fn `LookAt`
  (returns (Return :type Boolean))
  (`parent.LookAt`)
  (if (`self.Interactable`)
    (`PrimitiveComponent.SetCustomDepthStencilValue` (`self.StaticMesh`) 2)
    (return false)))

(fn `StopLookAt`
  (returns (Return :type Boolean))
  (`parent.StopLookAt`)
  (`PrimitiveComponent.SetCustomDepthStencilValue` (`self.StaticMesh`) 0)
  (return false))

(fn `UserConstructionScript`
  (`parent.UserConstructionScript`))