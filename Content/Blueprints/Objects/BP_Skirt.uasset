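; BP_Skirt is a collectible skirt object that the player can look at and interact with, built on a parent interactable class.
; Looking at it while interactable sets a custom depth stencil value for highlighting, which clears when the look ends.
; On BeginPlay it caches the first PC actor and its item enum.
; Interacting flags that enum's index in the PC's CollectedItems array, destroys the actor and plays a 2D voice line.
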(event `self.ReceiveBeginPlay`
  (`parent.ReceiveBeginPlay`)
  (`|ExecutionSequence`
    (:`then_0`
      (`PrimitiveComponent.SetRenderCustomDepth` (`self.StaticMesh`) true))
    (:`then_1`
      (bind _outactors (`GameplayStatics.GetAllActorsOfClass` "/Game/Blueprints/PC.PC_C"))
      (set `self.PC` (`|GetArrayItem` _outactors))
      (set `self.ThisItem` "NewEnumerator1"))))

(fn `AddToComputer`
  (`KismetArrayLibrary.Array_Set` (`/Game/Blueprints/PC.CollectedItems` (`self.PC`)) (`KismetMathLibrary.Conv_ByteToInt` (`self.ThisItem`)) true))

(fn `InteractWith`
  (returns (Return :type Boolean))
  (`self.AddToComputer`)
  (`self.K2_DestroyActor`)
  (set `self.Collected` true)
  (bind _returnvalue (`GameplayStatics.CreateSound2D` "/Game/SFX/After_Hours_VA_-_SkirtShirt.After_Hours_VA_-_SkirtShirt" 1.0 1.0 0.0 null))
  (`AudioComponent.Play` _returnvalue 0.0)
  (return false))

(fn `LookAt`
  (returns (Return :type Boolean))
  (`parent.LookAt`)
  (if (`self.Interactable`)
    (`PrimitiveComponent.SetCustomDepthStencilValue` (`self.StaticMesh`) 2)
    (return false)))

(fn `StopLookAt`
  (returns (Return :type Boolean))
  (`parent.StopLookAt`)
  (`PrimitiveComponent.SetCustomDepthStencilValue` (`self.StaticMesh`) 0)
  (return false))

(fn `UserConstructionScript`
  (`parent.UserConstructionScript`))