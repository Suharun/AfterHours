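; BP_PostItIts is an interactable post-it note pickup that shows its note on screen when used.
; BeginPlay creates a hidden PostItUI1 widget in the viewport.
; LookAt and StopLookAt extend parent behavior, toggling the mesh's custom depth stencil value as a highlight when interactable.
; InteractWith destroys the actor, sets Collected to false, reveals the widget and plays a 2D post-it voice sound.
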(event `self.ReceiveBeginPlay`
  (`parent.ReceiveBeginPlay`)
  (bind _returnvalue (`|CreateWidget` "/Game/UI/PostItUI/PostItUI1.PostItUI1_C"))
  (bind _output_get (set `self.UI Reference` _returnvalue))
  (`UserWidget.AddToViewport` _output_get 0)
  (`Widget.SetVisibility` _output_get "Hidden"))

(fn `InteractWith`
  (returns (Return :type Boolean))
  (`self.K2_DestroyActor`)
  (set `self.Collected` false)
  (`Widget.SetVisibility` (`self.UI Reference`) "Visible")
  (bind _returnvalue (`GameplayStatics.CreateSound2D` "/Game/SFX/After_Hours_VA_-_Subsequent_Postits.After_Hours_VA_-_Subsequent_Postits" 1.0 1.0 0.0 null))
  (`AudioComponent.Play` _returnvalue 0.0)
  (return false))

(fn `LookAt`
  (returns (Return :type Boolean))
  (`parent.LookAt`)
  (if (`self.Interactable`)
    (`PrimitiveComponent.SetCustomDepthStencilValue` (`self.StaticMesh`) 2)
    (return false)))

(fn `StopLookAt`
  (returns (Return :type Boolean))
  (`parent.StopLookAt`)
  (`PrimitiveComponent.SetCustomDepthStencilValue` (`self.StaticMesh`) 0)
  (return false))

(fn `UserConstructionScript`
  (`parent.UserConstructionScript`))