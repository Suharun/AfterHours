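; BP_Battery is an interactable pickup that recharges the player's flashlight.
; Overlap caches the BP_Player reference that InteractWith later uses.
; If the player has a flashlight below full charge, interacting adds BatteryAmmoValue to its meter, capped at 100, then destroys the battery and plays a 2D "battery found" sound.
; LookAt and StopLookAt toggle the mesh's custom depth stencil value, with LookAt gated by Interactable.
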(event `self.ReceiveActorBeginOverlap`
  (params (OtherActor :type "Actor Object Reference"))
  (`parent.ReceiveActorBeginOverlap` OtherActor)
  (bind _asbp_player (cast `/Game/Blueprints/BP_Player` OtherActor))
  (set `self.Player` _asbp_player))

(fn `InteractWith`
  (returns (Return :type Boolean))
  (bind _player (`self.Player`))
  (bind _flashlightreference (`/Game/Blueprints/BP_Player.FlashlightReference` _player))
  (bind _flashlightmeter (`/Game/Blueprints/Flashlight.FlashlightMeter` _flashlightreference))
  (if (`KismetSystemLibrary.IsValid` _player)
    (if (and (`/Game/Blueprints/BP_Player.HasFlashlight` _player) (< _flashlightmeter 100.0))
      (bind _output_get (set `/Game/Blueprints/Flashlight.FlashlightMeter` (+ (`self.Battery Ammo Value`) _flashlightmeter) _flashlightreference))
      (if (>= _output_get 100.0)
        (set `/Game/Blueprints/Flashlight.FlashlightMeter` 100.0 _flashlightreference))
      (`self.K2_DestroyActor`)
      (bind _returnvalue (`GameplayStatics.CreateSound2D` "/Game/SFX/After_Hours_VA_-_Battery_found_1.After_Hours_VA_-_Battery_found_1" 1.0 1.0 0.0 null))
      (`AudioComponent.Play` _returnvalue 0.0)
      (return false))))

(fn `LookAt`
  (returns (Return :type Boolean))
  (if (`self.Interactable`)
    (`PrimitiveComponent.SetCustomDepthStencilValue` (`self.StaticMesh`) 2)
    (return false)))

(fn `StopLookAt`
  (returns (Return :type Boolean))
  (`parent.StopLookAt`)
  (`PrimitiveComponent.SetCustomDepthStencilValue` (`self.StaticMesh`) 0)
  (return false))

(fn `UserConstructionScript`
  (`parent.UserConstructionScript`))