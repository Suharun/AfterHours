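; Interactable in-game PC that opens an on-screen menu with the mouse cursor and locks the player's look while in use.
; Overrides LookAt and StopLookAt to toggle a highlight through the mesh's custom depth stencil when interactable.
; InteractWith creates the menu widget; ClosePCMenu removes it plus any email or files widgets and restores look control.
; BeginPlay sizes a CollectedItems bool array from an enum, all false.
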(event `self.ReceiveBeginPlay`
  (bind _returnvalue (enumcount `/Game/Blueprints/E_CollectableItems`))
  (bind _collecteditems (`self.CollectedItems`))
  (`parent.ReceiveBeginPlay`)
  ;[1 1 1] Create array of bools for each collected item, set to false by default (for not collected)
  (`KismetArrayLibrary.Array_Resize` _collecteditems _returnvalue)
  (for _index (range (+ _returnvalue 1))
    (`KismetArrayLibrary.Array_Set` _collecteditems _index)))

(fn `ClosePCMenu`
  (bind _returnvalue (`GameplayStatics.GetPlayerController` 0))
  (bind _pcemailwidget (`self.PCEmailWidget`))
  (bind _pcfileswidget (`self.PCFilesWidget`))
  (`Widget.RemoveFromParent` (`self.PCMenuWidget`))
  (if (`KismetSystemLibrary.IsValid` _pcemailwidget)
    (`Widget.RemoveFromParent` _pcemailwidget))
  (if (`KismetSystemLibrary.IsValid` _pcfileswidget)
    (`Widget.RemoveFromParent` _pcfileswidget))
  (set `/Game/Blueprints/BP_Player.LockPlayerLookAround` false (`self.PlayerReference`))
  (set `PlayerController.bShowMouseCursor` false _returnvalue)
  (`Controller.SetIgnoreMoveInput` _returnvalue false))

(fn `InteractWith`
  (returns (Return :type Boolean))
  (bind _returnvalue (`GameplayStatics.GetPlayerController` 0))
  (bind _returnvalue_2 (`|CreateWidget` "/Game/UI/UI_PC_Interface.UI_PC_Interface_C" (`GameplayStatics.GetPlayerController` 0)))
  (bind _output_get (set `self.PCMenuWidget` _returnvalue_2))
  (`UserWidget.AddToViewport` _output_get 0)
  (set `PlayerController.bShowMouseCursor` true _returnvalue)
  (`Controller.SetIgnoreMoveInput` _returnvalue false)
  (bind _asbp_player (cast `/Game/Blueprints/BP_Player` (`GameplayStatics.GetPlayerCharacter` 0)))
  (bind _output_get_2 (set `self.PlayerReference` _asbp_player))
  (set `/Game/Blueprints/BP_Player.LockPlayerLookAround` true _output_get_2)
  (return false))

(fn `LookAt`
  (returns (Return :type Boolean))
  (`parent.LookAt`)
  (if (`self.Interactable`)
    (`PrimitiveComponent.SetCustomDepthStencilValue` (`self.StaticMesh`) 2)
    (return false)))

(fn `StopLookAt`
  (returns (Return :type Boolean))
  (`parent.StopLookAt`)
  (`PrimitiveComponent.SetCustomDepthStencilValue` (`self.StaticMesh`) 0)
  (return false))

(fn `UserConstructionScript`
  (`parent.UserConstructionScript`))