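; Base interactable object with a custom-depth highlight and a stub InteractWith function that returns false.
; BeginPlay enables custom depth on the mesh, and LookAt sets its stencil value to show the outline when Interactable is true.
; Tick clears the stencil through StopLookAt every frame, so the highlight lasts only while LookAt keeps being called.
; Overlap events track whether BP_Player is close enough, though nothing here reads that flag.
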(event `self.ReceiveBeginPlay`
  (`PrimitiveComponent.SetRenderCustomDepth` (`self.StaticMesh`) true))

(event `self.ReceiveActorBeginOverlap`
  (params (OtherActor :type "Actor Object Reference"))
  ;[1 1 1] Check if actor overlap is player (cast will succeed)
  (cast `/Game/Blueprints/BP_Player` OtherActor)
  (set `self.PlayerCloseEnough` true))

(event `self.ReceiveActorEndOverlap`
  (params (OtherActor :type "Actor Object Reference"))
  ;[1 1 1] Check if actor overlap is player (cast will succeed)
  (cast `/Game/Blueprints/BP_Player` OtherActor)
  (set `self.PlayerCloseEnough` false))

(event `self.ReceiveTick`
  (params (DeltaSeconds :type "Float (single-precision)"))
  (`self.ResetOutline`))

(fn `InteractWith`
  (returns (Return :type Boolean))
  (return false))

(fn `LookAt`
  (returns (Return :type Boolean))
  (if (`self.Interactable`)
    (`PrimitiveComponent.SetCustomDepthStencilValue` (`self.StaticMesh`) 2)
    (return false)))

(fn `ResetOutline`
  (`self.StopLookAt`))

(fn `StopLookAt`
  (returns (Return :type Boolean))
  (`PrimitiveComponent.SetCustomDepthStencilValue` (`self.StaticMesh`) 0)
  (return false))

(fn `UserConstructionScript`)