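; First-person player Blueprint handling movement, look, flashlight use and interaction with world objects.
; A per-tick camera line trace stores the BP_Interactable_Object under view via I_Interactable and calls LookAt; releasing PickUp interacts with it.
; Pressing PickUp attaches the level's first Flashlight actor to the camera when close enough, after which ToggleFlashlight switches it and its drain.
; Look input respects a lock flag, and ExitMenu closes a looked-at PC's menu.
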(event `self.ReceiveTick`
  (params (DeltaSeconds :type "Float (single-precision)"))
  (`self.LineTrace`))

(event `self.ReceiveBeginPlay`
  ;[1 0.3267 0.9448] Player does not have the flashlight by default
  (`SceneComponent.SetVisibility` (`self.FlashlightModel`) false false)
  (set `self.HasFlashlight` false)
  (bind _outactors (`GameplayStatics.GetAllActorsOfClass` "/Game/Blueprints/Flashlight.Flashlight_C"))
  (set `self.FlashlightReference` (`|GetArrayItem` _outactors)))

(event `InputAction|ToggleFlashlight`
  (params (Key :type "Key Structure"))
  (bind _flashlightreference (`self.FlashlightReference`))
  ;[0.8702 0.2124 1] If the player has the flashlight and presses the 'F' key then toggle
  (:`Pressed`
    (if (`self.HasFlashlight`)
      (`/Game/Blueprints/Flashlight.ToggleFlashlight` _flashlightreference)
      (set `/Game/Blueprints/Flashlight.DrainOn` (not (`/Game/Blueprints/Flashlight.DrainOn` _flashlightreference)) _flashlightreference))))

(event `InputAction|PickUp`
  (params (Key :type "Key Structure"))
  ;[0.6999 0.3001 1] Pick up items with 'E'
  (:`Pressed`
    (set `self.PickUp` true)
    (`self.AttemptFlashlightPickup`))
  (:`Released`
    (set `self.PickUp` false)
    ;[1 1 1] Interact with interactable object being looked at (if any)
    (if (`KismetSystemLibrary.IsValid` (`self.LookAtObject`))
      (`/Game/Blueprints/I_Interactable.InteractWith` (`self.LookAtObject`)))))

(event `InputAxis|Forward`
  (params (AxisValue :type "Float (single-precision)"))
  ;[1 1 1] Movement
  (`self.AddMovementInput` (`self.GetActorForwardVector`) AxisValue))

(event `InputAxis|Right`
  (params (AxisValue :type "Float (single-precision)"))
  ;[1 1 1] Movement
  (`self.AddMovementInput` (`self.GetActorRightVector`) AxisValue))

(event `InputAxis|Lookright`
  (params (AxisValue :type "Float (single-precision)"))
  ;[1 1 1] Look around
  (if (not (`self.LockPlayerLookAround`))
    (`self.AddControllerYawInput` AxisValue)))

(event `InputAxis|Lookup`
  (params (AxisValue :type "Float (single-precision)"))
  ;[1 1 1] Look around
  (if (not (`self.LockPlayerLookAround`))
    (`self.AddControllerPitchInput` AxisValue)))

(event `InputAction|ExitMenu`
  (params (Key :type "Key Structure"))
  (:`Released`
    ;[1 1 1] Check if lookAtObject was PC
    (bind _aspc (cast `/Game/Blueprints/PC` (`self.LookAtObject`)))
    (`/Game/Blueprints/PC.ClosePCMenu` _aspc)))

(fn `AttemptFlashlightPickup`
  ;[0.8477 0.2916 1] Checks if the player already has the flashlight and if they are close enough to pick it up
  (if (`self.HasFlashlight`)
    _
    (elif (`/Game/Blueprints/Flashlight.PlayerCloseEnough` (`self.FlashlightReference`))
      (`/Game/Blueprints/Flashlight.Pickup` (`self.FlashlightReference`) (`self.Camera`) self))))

(fn `LineTrace`
  (bind _camera (`self.Camera`))
  (bind _returnvalue (`SceneComponent.K2_GetComponentLocation` _camera))
  (set `self.LookAtObject` null)
  ;[1 1 1] Draw a line towards where player is looking
  (bind _outhit (`KismetSystemLibrary.LineTraceSingle` _returnvalue (+ _returnvalue (* (`SceneComponent.GetForwardVector` _camera) (`self.LookDist`))) "TraceTypeQuery1"))
  (bind (_bblockinghit _binitialoverlap _time _distance _location _impactpoint _normal _impactnormal _physmat _hitactor) (`GameplayStatics.BreakHitResult` _outhit))
  ;[1 1 1] Does the actor being looked at implement 'interactable' interface?
  (if (`KismetSystemLibrary.DoesImplementInterface` _hitactor "/Game/Blueprints/I_Interactable.I_Interactable_C")
    (bind _asbp_interactable_object (cast `/Game/Blueprints/BP_Interactable_Object` _hitactor))
    (bind _output_get (set `self.LookAtObject` _asbp_interactable_object))
    (`/Game/Blueprints/BP_Interactable_Object.LookAt` _output_get)))

(fn `UserConstructionScript`
  (set `self.PickUp` false))