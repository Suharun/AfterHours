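; Interactable door Blueprint that swings open when used, optionally requiring the player to carry a key.
; InteractWith checks the BP_Player cached on overlap, playing an unlock or need-a-key sound, and sets Open.
; Tick then steps the mesh yaw to about 150 degrees, while leaving InteractZone snaps the rotation back without resetting Open or OpenStatus.
; LookAt and StopLookAt toggle a custom-depth stencil highlight on the mesh.
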(event `self.ReceiveActorBeginOverlap`
  (params (OtherActor :type "Actor Object Reference"))
  (`parent.ReceiveActorBeginOverlap` OtherActor)
  (bind _asbp_player (cast `/Game/Blueprints/BP_Player` OtherActor))
  (set `self.Player` _asbp_player))

(event `self.ReceiveTick`
  (params (DeltaSeconds :type "Float (single-precision)"))
  (`parent.ReceiveTick` DeltaSeconds)
  (if (`self.Open`)
    (if (<= (`self.OpenStatus`) 150.0)
      (bind _output_get (set `self.OpenStatus` (+ (`self.OpenStatus`) (`self.OpeningRate`))))
      (`SceneComponent.K2_SetRelativeRotation` (`self.StaticMesh`) (`KismetMathLibrary.MakeRotator` 0.0 0.0 _output_get) false false)
      (if (>= (`self.OpenStatus`) 150.0)
        (set `self.Opened` true)))))

(event `self.InteractZone.OnComponentEndOverlap`
  (params (OverlappedComponent :type "PrimitiveComponent Object Reference") (OtherActor :type "Actor Object Reference") (OtherComp :type "PrimitiveComponent Object Reference") (OtherBodyIndex :type Integer))
  (cast `/Game/Blueprints/BP_Player` OtherActor)
  (`SceneComponent.K2_SetRelativeRotation` (`self.StaticMesh`) (`KismetMathLibrary.MakeRotator` 0.0) false false)
  (set `self.Opened` false))

(fn `InteractWith`
  (returns (Return :type Boolean))
  (bind _player (`self.Player`))
  (if (`self.Open`)
    _
    (elif (`self.NeedsKey`)
      (`/Engine/EditorBlueprintResources/StandardMacros.IsValid` _player
        (:`Is Valid`
          (if (`/Game/Blueprints/BP_Player.HasKey` _player)
            (bind _returnvalue (`GameplayStatics.CreateSound2D` "/Game/SFX/DoorLock.DoorLock" 1.0 1.0 0.0 null))
            (`AudioComponent.Play` _returnvalue 0.0)
            (`self.Open Door`)
            (return false)
            (else
              (bind _returnvalue_2 (`GameplayStatics.CreateSound2D` "/Game/SFX/After_Hours_VA_-_Need_a_Key.After_Hours_VA_-_Need_a_Key" 1.0 1.0 0.0 null))
              (`AudioComponent.Play` _returnvalue_2 0.0)))))
      (else
        (set `self.Open` true)))))

(fn `LookAt`
  (returns (Return :type Boolean))
  (`parent.LookAt`)
  (if (`self.Interactable`)
    (`PrimitiveComponent.SetCustomDepthStencilValue` (`self.StaticMesh`) 2)
    (return false)))

(fn `Open Door`
  (set `self.Open` true))

(fn `StopLookAt`
  (returns (Return :type Boolean))
  (`parent.StopLookAt`)
  (`PrimitiveComponent.SetCustomDepthStencilValue` (`self.StaticMesh`) 0)
  (return false))

(fn `UserConstructionScript`
  (`parent.UserConstructionScript`))